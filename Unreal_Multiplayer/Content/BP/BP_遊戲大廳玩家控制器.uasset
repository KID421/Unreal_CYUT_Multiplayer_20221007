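; Player controller for the game lobby (遊戲大廳) that sets up the local player's UI and pawn.
; On BeginPlay, only for the local controller, it adds the BW_遊戲大廳 widget to the viewport, shows the mouse cursor and calls 生成角色控制器.
; That event spawns BP_角色控制器 at the transform of the PlayerStart returned by GetActorOfClass, then possesses it.
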(event Custom|生成角色控制器
  (bind _returnvalue (Actor|GetActorOfClass "/Script/Engine.PlayerStart")) ; 透過類別取得物件：地圖上有的物件才可以抓取
  (bind _returnvalue_2 (Game|SpawnActorfromClass "/Game/BP/BP_角色控制器.BP_角色控制器_C" (Transformation|GetActorTransform _returnvalue) "Undefined" 0 0)) ; Create Actor 建立物件
  (Pawn|Possess _returnvalue_2) ; 具體化：將物件具體化於伺服器內
)

(event EventBeginPlay
  (if (Pawn|IsLocalPlayerController)
    (bind _returnvalue (UserInterface|CreateWidget "/Game/BP/BW_遊戲大廳.BW_遊戲大廳_C"))
    (UserInterface|Viewport|AddtoViewport _returnvalue 0)
    (Variables|Default|SetbShowMouseCursor true)
    (CallFunction|生成角色控制器)))

(fn ConstructionScript)